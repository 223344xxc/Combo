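; Dragon monster Blueprint that configures a high-health enemy with an overhead HP widget.
; BeginPlay links the MonsterHp widget to this actor, then sets health, search range, attack and respawn delay, calling ResetAbility before the respawn value is assigned.
; Tick rotates the widget toward the BP_FPSCharacter found by a per-frame GetActorOfClass lookup.
; No combat or movement logic appears in these graphs.
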(event EventBeginPlay
  (bind _self self)
  (bind _asmonster_hp (Utilities|Casting|CastToMonsterHp (UserInterface|GetUserWidgetObject (Variables|Default|GetWidget))))
  (Variables|/Game/UI/MonsterHp.MonsterHp_C|SetOwner _asmonster_hp _self)
  (Variables|/Script/FPS.BP_Monster|SetMaxHp _self 1e+04)
  (Variables|Default|SetSurchDistance _self 2e+03)
  (Variables|Default|SetATK _self 2e+01)
  (Class|BPMonster|ResetAbility _self)
  (Variables|Default|SetReSpawnDelay _self 3e+02))

(event Collision|EventActorBeginOverlap
  (params (OtherActor :type Actor%20Object%20Reference)))

(event EventTick
  (params (DeltaSeconds :type Float%20%28single-precision%29))
  (bind _widget (Variables|Default|GetWidget))
  (bind _returnvalue (Actor|GetActorOfClass "/Game/Blueprints/BP_FPSCharacter.BP_FPSCharacter_C"))
  (Transformation|SetWorldRotation _widget (Math|Rotator|FindLookatRotation (Transformation|GetWorldLocation _widget) (Transformation|GetActorLocation _returnvalue)) false false))

(fn ConstructionScript)