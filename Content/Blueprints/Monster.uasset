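; Monster actor that carries a world-space widget component for its health display.
; On BeginPlay it casts the widget to MonsterHp and hands itself over as that widget's Owner.
; Every Tick it looks up the BP_FPSCharacter actor and rotates the widget to face it, billboard style, using a look-at rotation.
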(event EventBeginPlay
  (bind _asmonster_hp (Utilities|Casting|CastToMonsterHp (UserInterface|GetUserWidgetObject (Variables|Default|GetWidget))))
  (Variables|/Game/UI/MonsterHp.MonsterHp_C|SetOwner _asmonster_hp self))

(event Collision|EventActorBeginOverlap
  (params (OtherActor :type Actor%20Object%20Reference)))

(event EventTick
  (params (DeltaSeconds :type Float%20%28single-precision%29))
  (bind _widget (Variables|Default|GetWidget))
  (bind _returnvalue (Actor|GetActorOfClass "/Game/Blueprints/BP_FPSCharacter.BP_FPSCharacter_C"))
  (Transformation|SetWorldRotation _widget (Math|Rotator|FindLookatRotation (Transformation|GetWorldLocation _widget) (Transformation|GetActorLocation _returnvalue)) false false))

(fn ConstructionScript)